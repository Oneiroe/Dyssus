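; BPFootsteps is a prototype footstep Blueprint that plays a surface-dependent sound at the ground below the actor.
; Pressing the Run input while the actor is moving fires a single downward Visibility trace, and the hit's physical surface selects the sound played at the impact point.
; Only the default surface has a sound assigned, a Fire01 placeholder, and nothing repeats the sound per step.
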(event `InputAction|Run`
  (bind _returnvalue (`self.K2_GetActorLocation`))
  (:`Pressed`
    (if (> (`KismetMathLibrary.VSize` (`self.GetVelocity`)) 25.0)
      (bind (_outhit _returnvalue_2) (`KismetSystemLibrary.LineTraceSingle` _returnvalue (- _returnvalue (0.0 0.0 150.0)) "TraceTypeQuery1"))
      (if _returnvalue_2
        (`GameplayStatics.PlaySoundAtLocation` (select `EngineTypes.EPhysicalSurface` (`GameplayStatics.GetSurfaceType` _outhit) :`SurfaceType_Default` "/Game/StarterContent/Audio/Fire01.Fire01" :!type "SoundBase Object Reference") (`.Location` (`GameplayStatics.BreakHitResult` _outhit)))))))

(event `self.ReceiveBeginPlay`)

(event `self.ReceiveActorBeginOverlap`
  (params (OtherActor :type "Actor Object Reference")))

(event `self.ReceiveTick`
  (params (DeltaSeconds :type "Float (single-precision)")))

(fn `UserConstructionScript`)