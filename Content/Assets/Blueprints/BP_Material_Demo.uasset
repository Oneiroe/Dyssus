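; BP_Material_Demo is a display actor that demonstrates base color, roughness and metallic material parameters.
; Its construction script creates a dynamic material instance on each of three components, setting textures and parameters from the actor's variables.
; A ShowTexture flag switches the base color sample's texture.
; Text renders label the roughness and metallic samples with their values, truncated to three characters.
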(fn `UserConstructionScript`
  (bind _roughness (`self.Roughness`))
  (bind _metallic (`self.Metallic`))
  (bind _returnvalue (`PrimitiveComponent.CreateDynamicMaterialInstance` (`self.Base Color`) 0 null))
  (`MaterialInstanceDynamic.SetVectorParameterValue` _returnvalue "Color" (`self.BaseColor`))
  (`MaterialInstanceDynamic.SetTextureParameterValue` _returnvalue "Texture" (select `bool` (`self.Show texture`) :`false` "/Game/Assets/Textures/T_RoomTiles_M.T_RoomTiles_M" :`true` "/Game/Assets/Textures/T_CorrodedMetal_D.T_CorrodedMetal_D" :!type "Texture Object Reference"))
  (`MaterialInstanceDynamic.SetScalarParameterValue` _returnvalue "Roughness" 1.0)
  (bind _returnvalue_2 (`PrimitiveComponent.CreateDynamicMaterialInstance` (`self.RoughnessInternal`) 0 null))
  (`MaterialInstanceDynamic.SetTextureParameterValue` _returnvalue_2 "Texture" "/Game/Assets/Textures/T_ExampleLayers_Rubber01_D.T_ExampleLayers_Rubber01_D")
  (`MaterialInstanceDynamic.SetVectorParameterValue` _returnvalue_2 "Color" (struct :`R` 1.0 :`G` 0.399993 :`B` 0.105 :`A` 1.0))
  (`MaterialInstanceDynamic.SetScalarParameterValue` _returnvalue_2 "Roughness" _roughness)
  (`TextRenderComponent.SetText` (`self.TextRender2`) (`KismetStringLibrary.Concat_StrStr` "Roughness:  " (`KismetStringLibrary.GetSubstring` (`KismetStringLibrary.Conv_DoubleToString` _roughness) 0 3)))
  (bind _returnvalue_3 (`PrimitiveComponent.CreateDynamicMaterialInstance` (`self.MetallicInternal`) 0 null))
  (`MaterialInstanceDynamic.SetTextureParameterValue` _returnvalue_3 "Texture" "/Game/Assets/DUPLICATES/T_Metal_Painted01_D.T_Metal_Painted01_D")
  (`MaterialInstanceDynamic.SetScalarParameterValue` _returnvalue_3 "Metallic" _metallic)
  (`TextRenderComponent.SetText` (`self.TextRender3`) (`KismetStringLibrary.Concat_StrStr` "Metallic: " (`KismetStringLibrary.GetSubstring` (`KismetStringLibrary.Conv_DoubleToString` _metallic) 0 3))))